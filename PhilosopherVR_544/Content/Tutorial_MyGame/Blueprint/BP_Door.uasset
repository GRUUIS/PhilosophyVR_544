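; BP_Door is a hinged door that swings between closed and open yaw angles.
; StartMove and StopMove toggle a driving flag that gates the Tick update.
; While driving, Tick advances a clamped 0–1 alpha by DoorSpeed times delta time and lerps the HingePivot's relative yaw from it.
; Stopping holds the current angle, and reaching either limit does not clear the flag.
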(event `self.ReceiveTick`
  (params (DeltaSeconds :type "Float (single-precision)"))
  (if (`self.bDoorDriving`)
    (bind _output_get (set `self.DoorAlpha` (`KismetMathLibrary.FClamp` (+ (`self.DoorAlpha`) (* (`self.DoorSpeed`) (`GameplayStatics.GetWorldDeltaSeconds`))))))
    (`SceneComponent.K2_SetRelativeRotation` (`self.HingePivot`) (`KismetMathLibrary.MakeRotator` 0.0 0.0 (`KismetMathLibrary.Lerp` (`self.DoorClosedYaw`) (`self.DoorOpenYaw`) _output_get)) false false)))

(event `StartMove`
  (set `self.bDoorDriving` true))

(event `StopMove`
  (set `self.bDoorDriving` false))

(fn `UserConstructionScript`)