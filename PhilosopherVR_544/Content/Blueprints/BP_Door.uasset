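; Interactable hinged door that swings open one way and shows or hides a widget interaction prompt.
; StartMove plays a timeline that lerps the hinge pivot's yaw from closed to opened, triggers the door sound from an event track, and disables interaction when finished.
; The prompt starts hidden and is toggled through SetPromptVisible.
; An unconnected delta-time rotation approach remains, noted as abandoned in favor of animation.
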(event `StartMove`
  (bind (_direction _alpha) (`Timeline|TL_Door`)
    (:`Update`
      (`SceneComponent.K2_SetRelativeRotation` (`self.HingePivot`) (`KismetMathLibrary.MakeRotator` 0.0 0.0 (`KismetMathLibrary.Lerp` (`self.DoorClosedYaw`) (`self.DoorOpenedYaw`) _alpha)) false false))
    (:`Finished`
      (set `self.bInteractionEnabled` false))
    (:`SoundPlayTime`
      (`AudioComponent.Play` (`self.AC_DoorLoop`) 0.0))))

(event `self.ReceiveBeginPlay`
  (`SceneComponent.SetHiddenInGame` (`self.WC_InteractPrompt`) true false))

(fn `SetPromptVisible`
  (params (bVisible :type Boolean))
  (bind _wc_interactprompt (`self.WC_InteractPrompt`))
  (`SceneComponent.SetHiddenInGame` _wc_interactprompt (not bVisible) false)
  (`SceneComponent.SetVisibility` _wc_interactprompt bVisible false))

(fn `UserConstructionScript`)