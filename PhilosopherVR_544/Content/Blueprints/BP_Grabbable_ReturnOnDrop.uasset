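; Grabbable actor that returns its mesh to its BeginPlay world transform when dropped outside a range box.
; After a drop and a delay, it tests the mesh origin in the box's local space against the scaled box extent.
; For a simulating mesh, it stops physics, zeroes velocities, moves it home and briefly disables collision before waking physics again.
; A non-simulating mesh simply teleports home.
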(event `self.ReceiveBeginPlay`
  (set `self.Home_Mesh_World` (`SceneComponent.K2_GetComponentToWorld` (`self.Mesh`))))

(event `self.GrabComponent.OnDropped`
  (bind _mesh (`self.Mesh`))
  (`KismetSystemLibrary.Delay` (`self.ReturnDelay`))
  (bind _insiderange (`self.IsGrabRootInsideRange`))
  (if _insiderange
    _
    (elif (`SceneComponent.IsSimulatingPhysics` _mesh "None")
      (`PrimitiveComponent.SetSimulatePhysics` _mesh false)
      (`PrimitiveComponent.SetPhysicsLinearVelocity` _mesh (0.0 0.0 0.0) false "None")
      (`PrimitiveComponent.SetPhysicsAngularVelocityInDegrees` _mesh (0.0 0.0 0.0) false "None")
      (`SceneComponent.K2_SetWorldTransform` (`self.Mesh`) (`self.Home_Mesh_World`) false false)
      (`PrimitiveComponent.SetCollisionEnabled` _mesh "NoCollision")
      (`KismetSystemLibrary.Delay` (`self.ReenablePhysicsDelay`))
      (`PrimitiveComponent.SetCollisionEnabled` _mesh "QueryAndPhysics")
      (`PrimitiveComponent.SetSimulatePhysics` _mesh true)
      (`PrimitiveComponent.WakeRigidBody` _mesh "None")
      (else
        (`SceneComponent.K2_SetWorldTransform` (`self.Mesh`) (`self.Home_Mesh_World`) false true)))))

(fn `IsGrabRootInsideRange`
  (returns (InsideRange :type Boolean))
  (bind _rangebox (`self.RangeBox`))
  (return (and (<= (`KismetMathLibrary.Abs` (.x (`KismetMathLibrary.InverseTransformLocation` (`SceneComponent.K2_GetComponentToWorld` _rangebox) (`SceneComponent.K2_GetComponentLocation` (`self.Mesh`))))) (.x (`BoxComponent.GetScaledBoxExtent` _rangebox))) (<= (`KismetMathLibrary.Abs` (.y (`KismetMathLibrary.InverseTransformLocation` (`SceneComponent.K2_GetComponentToWorld` _rangebox) (`SceneComponent.K2_GetComponentLocation` (`self.Mesh`))))) (.y (`BoxComponent.GetScaledBoxExtent` _rangebox))) (<= (`KismetMathLibrary.Abs` (.z (`KismetMathLibrary.InverseTransformLocation` (`SceneComponent.K2_GetComponentToWorld` _rangebox) (`SceneComponent.K2_GetComponentLocation` (`self.Mesh`))))) (.z (`BoxComponent.GetScaledBoxExtent` _rangebox))))))

(fn `UserConstructionScript`)