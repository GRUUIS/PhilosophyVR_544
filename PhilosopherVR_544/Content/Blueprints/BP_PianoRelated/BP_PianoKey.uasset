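; BP_PianoKey is a VR piano key that plays its note and reports presses to a piano manager.
; When pressed while unlocked, the VR button passes the key ID and interacting component to the manager, then plays the note at the key's location.
; A trigger flag debounces presses, resetting after a short delay only when the note sound is valid.
; ShowHint and HideHint toggle a hint effect.
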(event `self.VRButton.OnButtonStateChanged`
  (params (ButtonState :type Boolean) (InteractingActor :type "Actor Object Reference") (InteractingComponent :type "PrimitiveComponent Object Reference"))
  (bind _notesound (`self.NoteSound`))
  (if (`self.bIsLocked`)
    _
    (elif ButtonState
      (if (not (`self.bAlreadyTriggered`))
        (set `self.bAlreadyTriggered` true)
        (`/Game/Blueprints/BP_PianoRelated/BP_PianoManager.HandleKeyPressed` (`self.PianoManagerRef`) (`self.KeyID`) InteractingComponent)
        (`KismetSystemLibrary.PrintString` "AFTER HandleKeyPressed")
        (if (`KismetSystemLibrary.IsValid` _notesound)
          (`KismetSystemLibrary.PrintString` (`KismetStringLibrary.Concat_StrStr` "ValidNoteSound" (`KismetSystemLibrary.GetDisplayName` _notesound)))
          (`GameplayStatics.PlaySoundAtLocation` _notesound (`self.K2_GetActorLocation`) (struct) 1.0 1.0 0.0 null null null null)
          (`KismetSystemLibrary.Delay` 0.1)
          (set `self.bAlreadyTriggered` false))))))

(fn `HideHint`
  (`ActorComponent.Deactivate` (`self.HintFX`)))

(fn `ShowHint`
  (bind _hintfx (`self.HintFX`))
  (`NiagaraComponent.ReinitializeSystem` _hintfx)
  (`ActorComponent.Activate` _hintfx false))

(fn `UserConstructionScript`)