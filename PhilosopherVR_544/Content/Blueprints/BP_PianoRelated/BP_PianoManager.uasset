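; Manager for a VR piano minigame where the player plays a song's keys in order, guided by a hint on the target key.
; Correct presses advance the song with shorter per-key timers and stronger haptics on the playing hand.
; Wrong presses and timeouts add mistakes that darken the HUD, and reaching the limit restarts the song after a delay.
; Completing the song clears the hints and darkness.
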(event `self.ReceiveBeginPlay`
  (if (> (`KismetArrayLibrary.Array_Length` (`self.SongKeys`)) 0)
    (set `self.CurrentTargetKeyID` (`|GetArrayItem` (`self.SongKeys`)))
    (`self.UpdateCurrentTargetKeyRef`)
    (`self.RefreshHints`)
    (bind _returnvalue (`|CreateWidget` "/Game/Blueprints/BP_PianoRelated/WBP_PianoHUD.WBP_PianoHUD_C"))
    (bind _output_get (set `self.PianoHUDRef` _returnvalue))
    (`UserWidget.AddToViewport` _output_get 0)
    (`/Game/Blueprints/BP_PianoRelated/WBP_PianoHUD.SetDarknessAlpha` _output_get 0.0)))

(event `Penalty Reset Delayed`
  (set `self.bInPenaltyReset` true)
  (`self.UpdateDarknessFromMistakes`)
  (`KismetSystemLibrary.Delay` 2.0)
  (`self.StartOver`))

(fn `ClearAllHints`
  (for _array_element (`self.PianoKeys`)
    (`/Engine/EditorBlueprintResources/StandardMacros.IsValid` _array_element
      (:`Is Valid`
        (`/Game/Blueprints/BP_PianoRelated/BP_PianoKey.HideHint` _array_element)))))

(fn `CompleteSong`
  (bind _currenttargetkeyref (`self.CurrentTargetKeyRef`))
  (bind _pianohudref (`self.PianoHUDRef`))
  (`KismetSystemLibrary.K2_ClearAndInvalidateTimerHandle` (`self.CurrentKeyTimerHandle`))
  (set `self.bHasCompleted` true)
  (`KismetSystemLibrary.PrintString` "Song Completed")
  (`/Engine/EditorBlueprintResources/StandardMacros.IsValid` _currenttargetkeyref
    (:`Is Valid`
      (`/Game/Blueprints/BP_PianoRelated/BP_PianoKey.HideHint` _currenttargetkeyref)
      (`self.ClearAllHints`) ; Just in case...
      (bind _output_get (set `self.DarknessAlpha` 0.0))
      (`/Engine/EditorBlueprintResources/StandardMacros.IsValid` _pianohudref
        (:`Is Valid`
          (`/Game/Blueprints/BP_PianoRelated/WBP_PianoHUD.SetDarknessAlpha` _pianohudref _output_get))))))

(fn `GetCorrectKeyHapticIntensity`
  (returns (ReturnValue :type "Float (double-precision)"))
  (return (`KismetMathLibrary.Lerp` 0.1 1.0 (`KismetMathLibrary.FClamp` (/ (`KismetMathLibrary.Conv_IntToDouble` (+ (`self.CurrentIndex`) 1)) (`KismetMathLibrary.Conv_IntToDouble` (`KismetMathLibrary.Max` (`KismetArrayLibrary.Array_Length` (`self.SongKeys`)) 1)))))) ; ReturnValue = Lerp(0.25, 1.0, Clamp((CurrentIndex + 1) / Max(SongKeys.Length, 1), 0, 1))
)

(fn `HandleKeyPressed`
  (params (PressedKeyID :type Name) (InteractingComponent :type "PrimitiveComponent Object Reference"))
  (if (not (`self.bHasCompleted`))
    (if (not (`self.bHasStarted`))
      (set `self.bHasStarted` true)
      (`self.StartTargetKeyTimer`))
    (if (== PressedKeyID (`self.CurrentTargetKeyID`))
      (`KismetSystemLibrary.PrintString` "Right Key~~~")
      (bind _returnvalue (`self.GetCorrectKeyHapticIntensity`))
      (`self.TriggerCorrectKeyHaptic` InteractingComponent _returnvalue)
      (`KismetSystemLibrary.K2_ClearAndInvalidateTimerHandle` (`self.CurrentKeyTimerHandle`))
      (set `self.CurrentIndex` (+ (`self.CurrentIndex`) 1))
      (if (>= (`self.CurrentIndex`) (`KismetArrayLibrary.Array_Length` (`self.SongKeys`)))
        (`self.CompleteSong`)
        (else
          (set `self.CurrentTargetKeyID` (`|GetArrayItem` (`self.SongKeys`) (`self.CurrentIndex`))) ; 系统现在已经切到了下一个该按的键
          (`self.UpdateCurrentTargetKeyRef`)
          (`self.RefreshHints`)
          (`self.StartTargetKeyTimer`)))
      (else
        (`KismetSystemLibrary.PrintString` "Wrong Key!!!!!!")
        (`self.RegisterMistake` 1) ; 错了以后，目标键不变，提示也不变，玩家必须继续对着当前提示键弹对
      ))))

(fn `OnTargetKeyTimerExpired`
  (if (and (== (`self.bHasCompleted`) false) (== (`self.bInPenaltyReset`) false))
    (`self.RegisterMistake` 1)
    (if (and (== (`self.bHasCompleted`) false) (== (`self.bInPenaltyReset`) false))
      (`self.StartTargetKeyTimer`))))

(fn `RefreshHints`
  (bind _previoustargetkeyref (`self.PreviousTargetKeyRef`))
  (bind _currenttargetkeyref (`self.CurrentTargetKeyRef`))
  (`/Engine/EditorBlueprintResources/StandardMacros.IsValid` _previoustargetkeyref
    (:`Is Valid`
      (`/Game/Blueprints/BP_PianoRelated/BP_PianoKey.HideHint` _previoustargetkeyref))
    (:`Is Not Valid`
      _))
  (`/Engine/EditorBlueprintResources/StandardMacros.IsValid` _currenttargetkeyref
    (:`Is Valid`
      (`/Game/Blueprints/BP_PianoRelated/BP_PianoKey.ShowHint` _currenttargetkeyref))
    (:`Is Not Valid`
      _))
  (set `self.PreviousTargetKeyRef` _currenttargetkeyref))

(fn `RegisterMistake`
  (params (MistakeAmount :type Integer :default 1))
  (if (`self.bHasCompleted`)
    _
    (elif (not (`self.bInPenaltyReset`))
      (bind _output_get (set `self.MistakeCount` (+ (`self.MistakeCount`) MistakeAmount)))
      (`self.UpdateDarknessFromMistakes`)
      (if (>= _output_get (`self.MaxMistakes`))
        (`self.Penalty Reset Delayed`)))))

(fn `StartOver`
  (bind _songkeys (`self.SongKeys`))
  (bind _pianohudref (`self.PianoHUDRef`))
  (`KismetSystemLibrary.K2_ClearAndInvalidateTimerHandle` (`self.CurrentKeyTimerHandle`))
  (set `self.bInPenaltyReset` true)
  (set `self.MistakeCount` 0)
  (set `self.CurrentIndex` 0)
  (set `self.bHasStarted` false)
  (set `self.bHasCompleted` false)
  (`self.ClearAllHints`)
  (set `self.PreviousTargetKeyRef` null)
  (set `self.CurrentTargetKeyRef` null)
  (if (> (`KismetArrayLibrary.Array_Length` _songkeys) 0)
    (set `self.CurrentTargetKeyID` (`|GetArrayItem` _songkeys))
    (`self.UpdateCurrentTargetKeyRef`)
    (`self.RefreshHints`))
  (set `self.bInPenaltyReset` false)
  (bind _output_get (set `self.DarknessAlpha` 0.0))
  (`/Engine/EditorBlueprintResources/StandardMacros.IsValid` _pianohudref
    (:`Is Valid`
      (`/Game/Blueprints/BP_PianoRelated/WBP_PianoHUD.SetDarknessAlpha` _pianohudref _output_get))))

(fn `StartTargetKeyTimer`
  (`KismetSystemLibrary.K2_ClearAndInvalidateTimerHandle` (`self.CurrentKeyTimerHandle`)) ; 每次目标键变化，都先把上一个计时器关掉。
  (bind _output_get (set `self.CurrentKeyTimeLimit` (`KismetMathLibrary.FMax` (- (`self.BaseKeyTimeLimit`) (* (`KismetMathLibrary.Conv_IntToDouble` (`self.CurrentIndex`)) (`self.TimeLimitDecreasePerSuccess`))) (`self.MinKeyTimeLimit`)))) ; 随着 CurrentIndex 增加，时间会越来越短，但不会低于最小值
  (bind _returnvalue (`KismetSystemLibrary.K2_SetTimer` null "OnTargetKeyTimerExpired" _output_get))
  (set `self.CurrentKeyTimerHandle` _returnvalue))

(fn `TriggerCorrectKeyHaptic`
  (params (InteractingComponent :type "PrimitiveComponent Object Reference") (HapticIntensity :type "Float (double-precision)"))
  (bind _returnvalue (`KismetSystemLibrary.GetDisplayName` InteractingComponent))
  (`/Engine/EditorBlueprintResources/StandardMacros.IsValid` InteractingComponent
    (:`Is Valid`
      (bind _asvrpawn (cast `/Game/VRTemplate/Blueprints/VRPawn` (`GameplayStatics.GetPlayerPawn` 0)))
      (if (`KismetStringLibrary.Contains` _returnvalue "Sphere_Piano_L")
        (`/Game/VRTemplate/Blueprints/VRPawn.PlayPianoHapticLeft` _asvrpawn HapticIntensity)
        (elif (`KismetStringLibrary.Contains` _returnvalue "Sphere_Piano_R")
          (`/Game/VRTemplate/Blueprints/VRPawn.PlayPianoHapticRight` _asvrpawn HapticIntensity))))))

(fn `UpdateCurrentTargetKeyRef`
  (set `self.CurrentTargetKeyRef` null)
  (for _array_element (`self.PianoKeys`)
    (if (== (`/Game/Blueprints/BP_PianoRelated/BP_PianoKey.KeyID` _array_element) (`self.CurrentTargetKeyID`))
      (set `self.CurrentTargetKeyRef` _array_element))))

(fn `UpdateDarknessFromMistakes`
  (bind _pianohudref (`self.PianoHUDRef`))
  (bind _output_get (set `self.DarknessAlpha` (/ (`KismetMathLibrary.Conv_IntToDouble` (`self.MistakeCount`)) (`KismetMathLibrary.Conv_IntToDouble` (`self.MaxMistakes`)))))
  (`/Engine/EditorBlueprintResources/StandardMacros.IsValid` _pianohudref
    (:`Is Valid`
      (`/Game/Blueprints/BP_PianoRelated/WBP_PianoHUD.SetDarknessAlpha` _pianohudref _output_get))))

(fn `UserConstructionScript`)